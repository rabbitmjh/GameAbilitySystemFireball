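; Base projectile actor from the ToonProjectiles pack that spawns flash and hit effects and applies damage on impact.
; On BeginPlay, it requires a Character instigator, disables mutual move collision with it, plays the flash and self-destructs after a short lifetime.
; A sphere hit spawns the impact effect, optionally normal-aligned, turns off the light, then after a delay applies negative damage and destroys the actor.
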(event `self.ReceiveBeginPlay`
  (bind _sphere (`self.Sphere`))
  (bind _returnvalue (`self.GetInstigator` self))
  (bind `_as캐릭터` (cast `Character` _returnvalue))
  (`PrimitiveComponent.IgnoreComponentWhenMoving` (`Character.CapsuleComponent` `_as캐릭터`) _sphere true)
  (`PrimitiveComponent.IgnoreActorWhenMoving` _sphere _returnvalue true)
  (`NiagaraFunctionLibrary.SpawnSystemAtLocation` (`self.Flash effect`) (`self.K2_GetActorLocation`) (`self.K2_GetActorRotation`) (`self.Scale`))
  (`KismetSystemLibrary.Delay` 2.0)
  (`self.K2_DestroyActor` :!label _label))

(event `self.Sphere.OnComponentHit`
  (params (HitComponent :type "PrimitiveComponent Object Reference") (OtherActor :type "Actor Object Reference") (OtherComp :type "PrimitiveComponent Object Reference") (NormalImpulse :type "Vector Structure") (Hit :type "HitResult Structure (by ref)"))
  (bind (_bblockinghit _binitialoverlap _time _distance _location _impactpoint _normal _impactnormal _physmat _hitactor) (`GameplayStatics.BreakHitResult` Hit))
  (if (`self.Use zero rotation`)
    (set `self.Rotation` (struct))
    (else
      (set `self.Rotation` (`KismetMathLibrary.MakeRotFromX` _impactnormal))))
  (`NiagaraFunctionLibrary.SpawnSystemAtLocation` (`self.Hit effect`) _location (`self.Rotation`) (`self.Scale`))
  (`LightComponent.SetIntensity` (`self.PointLight`) 0.0)
  (`KismetSystemLibrary.Delay` (`self.Projectile hit destroy delay`))
  (`GameplayStatics.ApplyDamage` _hitactor -10.0)
  (goto _label))

(fn `UserConstructionScript`)